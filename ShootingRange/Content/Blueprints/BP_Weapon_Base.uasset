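; Base weapon Blueprint that attaches itself to the player's hand when interacted with, unless already attached.
; AttachToHand sets a fixed relative rotation, snaps the weapon to the AttachWeaponSocket on the player's mesh, and sets IsAttached.
; GetFirstPersonMesh finds that mesh by looping over all child components of player 0's root and returning the final element, with no name or type check.
; Debug prints trace the interaction and attachment.
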(event `self.Interact`
  (`KismetSystemLibrary.PrintString` "Called blueprint interact!!" true true (struct :`G` 0.66 :`B` 1.0 :`A` 1.0) 5.0)
  (if (not (`self.IsAttached`))
    (`self.AttachToHand`)))

(fn `AttachToHand`
  (bind (_returnvalue _array_index) (`self.GetFirstPersonMesh`))
  (`self.K2_SetActorRelativeRotation` (struct :`Pitch` 83.0 :`Yaw` 90.0 :`Roll` 90.0))
  (`self.K2_AttachToComponent` _returnvalue "AttachWeaponSocket" "SnapToTarget" "KeepRelative" "KeepWorld")
  (`KismetSystemLibrary.PrintString` (`KismetStringLibrary.Conv_IntToString` _array_index) true true (struct :`G` 0.66 :`B` 1.0 :`A` 1.0) 5.0)
  (`KismetSystemLibrary.PrintString` (`KismetSystemLibrary.GetDisplayName` _returnvalue) true true (struct :`G` 0.66 :`B` 1.0 :`A` 1.0) 5.0)
  (bind _output_get (set `self.IsAttached` true))
  (`KismetSystemLibrary.PrintString` (`KismetStringLibrary.Conv_BoolToString` _output_get)))

(fn `GetFirstPersonMesh`
  (returns (ReturnValue :type "SceneComponent Object Reference") (`Array Index` :type Integer))
  (for (_array_element _array_index) (`SceneComponent.GetChildrenComponents` (`Actor.RootComponent` (`GameplayStatics.GetPlayerCharacter` 0)) true)
    _)
  (return _array_element _array_index))

(fn `UserConstructionScript`)