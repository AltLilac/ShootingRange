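; Gun Blueprint that handles automatic fire and reloading from player input, with sounds and debug prints but no projectile or hit logic.
; Holding Fire runs a self-restarting timer, paced by RoundsPerMinute, that spends a bullet per shot after each delay.
; An enum state gates both actions: reload starts only from idle and refills after ReloadTime, unless firing has changed the state meanwhile.
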(event `InputAction|Fire`
  (params (Key :type "Key Structure"))
  (:`Pressed`
    (set `self.FireButtonDown` true)
    (`self.StartFire`))
  (:`Released`
    (set `self.FireButtonDown` false)))

(event `InputAction|Reload`
  (params (Key :type "Key Structure"))
  (:`Pressed`
    (`self.StartReload`)))

(event `self.ReceiveBeginPlay`
  (`self.SetFireDelay`))

(fn `Fire`
  (`KismetSystemLibrary.PrintString` "Fire")
  (set `self.CurrentBullet` (- (`self.CurrentBullet`) 1))
  (`KismetSystemLibrary.PrintString` (`KismetStringLibrary.Conv_IntToString` (`self.CurrentBullet`)))
  (set `self.GunState` "NewEnumerator1")
  (`GameplayStatics.PlaySoundAtLocation` "/Game/StarterContent/Audio/Explosion02.Explosion02" (`self.K2_GetActorLocation`) (struct) 1.0 1.0 0.0 null null null)
  (`self.StartFire`))

(fn `Reload`
  (if (`|EnumEquality` (`self.GunState`) "NewEnumerator0")
    (set `self.CurrentBullet` (`self.MaxBullet`))
    (`KismetSystemLibrary.PrintString` "Reload Complete")
    (set `self.GunState` "NewEnumerator1")))

(fn `SetFireDelay`
  (set `self.FireDelay` (/ 1.0 (`KismetMathLibrary.Conv_IntToDouble` (/ (`self.RoundsPerMinute`) 60)))))

(fn `StartFire`
  (if (`self.FireButtonDown`)
    (if (> (`self.CurrentBullet`) 0)
      (if (`|EnumInequality` (`self.GunState`) "NewEnumerator2")
        (set `self.GunState` "NewEnumerator2")
        (`KismetSystemLibrary.K2_SetTimer` null "Fire" (`self.FireDelay`))))))

(fn `StartReload`
  (if (>= (`self.CurrentBullet`) (`self.MaxBullet`))
    _
    (elif (`|EnumEquality` (`self.GunState`) "NewEnumerator1")
      (set `self.GunState` "NewEnumerator0")
      (`KismetSystemLibrary.PrintString` "Reloading")
      (`GameplayStatics.PlaySoundAtLocation` "/Game/StarterContent/Audio/Collapse01.Collapse01" (`self.K2_GetActorLocation`) (struct) 1.0 1.0 0.0 null null null)
      (`KismetSystemLibrary.K2_SetTimer` null "Reload" (`self.ReloadTime`)))))

(fn `UserConstructionScript`)